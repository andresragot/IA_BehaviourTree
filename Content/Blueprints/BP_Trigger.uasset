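; BP_Trigger is a trigger volume that tracks which foe actors are currently inside it.
; On actor begin overlap it casts to BP_Actor and, if the enum value is Foe, adds it uniquely to ArrayEnemies.
; When an actor stops overlapping its Box component, the same check removes it from the array.
; Print statements log entries, exits and failed casts for debugging.
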(event `self.ReceiveActorBeginOverlap`
  (params (OtherActor :type "Actor Object Reference"))
  (`KismetSystemLibrary.PrintString` "Entró algo")
  (bind _asbp_actor (cast `/Game/Blueprints/BP_Actor` OtherActor)
    (:`then`
      (switch `/Game/Blueprints/Enums/Enum_Actors` (`/Game/Blueprints/BP_Actor.Enum_Value` _asbp_actor)
        (:`NewEnumerator1`
          (`KismetSystemLibrary.PrintText` "Se metió")
          (`KismetArrayLibrary.Array_AddUnique` (`self.ArrayEnemies`) _asbp_actor))))
    (:`CastFailed`
      (`KismetSystemLibrary.PrintString` "Failed"))))

(event `self.Box.OnComponentEndOverlap`
  (params (OverlappedComponent :type "PrimitiveComponent Object Reference") (OtherActor :type "Actor Object Reference") (OtherComp :type "PrimitiveComponent Object Reference") (OtherBodyIndex :type Integer))
  (`KismetSystemLibrary.PrintString` "salió algo")
  (bind _asbp_actor (cast `/Game/Blueprints/BP_Actor` OtherActor))
  (switch `/Game/Blueprints/Enums/Enum_Actors` (`/Game/Blueprints/BP_Actor.Enum_Value` _asbp_actor)
    (:`NewEnumerator1`
      (`KismetSystemLibrary.PrintString` "Se salió")
      (`KismetArrayLibrary.Array_RemoveItem` (`self.ArrayEnemies`) _asbp_actor))))

(fn `UserConstructionScript`)